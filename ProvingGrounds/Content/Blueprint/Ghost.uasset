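; Ghost actor that animates the opacity of a translucent ghostly material so that it fades and pulses.
; The construction script creates dynamic material instances for the main mesh and for an Occluder that uses a depth mask material.
; On BeginPlay a timeline starts at a random time, varying the phase per instance, and drives the ghost material's maximum and minimum opacity, scaled by OpacityMax and PulseStrength.
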(event EventBeginPlay
  (Utilities|FlowControl|Sequence
    (:then_0
      (bind (_direction _opacitymain _opacitypulse) (Timeline|Timeline_0 SetNewTime)
        (:Update
          (Rendering|Material|SetScalarParameterValue (Variables|Default|GetGhostMat_Inst) "OpacityMax" (* _opacitymain (Variables|Default|GetOpacityMax)) :!class /Script/Engine.MaterialInstanceDynamic)
          (Rendering|Material|SetScalarParameterValue (Variables|Default|GetGhostMat_Inst) "OpacityMin" (Math|Float|MapRangeClamped _opacitypulse 0.0 1.0 (- 1.0 (Variables|Default|GetPulseStrength)) 1.0) :!class /Script/Engine.MaterialInstanceDynamic))))
    (:then_1
      (Timeline|Timeline_0 Play))))

(event EventTick
  (params (DeltaSeconds :type Float%20%28single-precision%29)))

(event Collision|EventActorBeginOverlap
  (params (OtherActor :type Actor%20Object%20Reference)))

(fn ConstructionScript
  (bind _returnvalue (Rendering|Material|CreateDynamicMaterialInstance (Variables|Default|GetMainMesh) 0 "/Game/Assets/Materials/ghastly_transluscent.ghastly_transluscent" :!class /Script/Engine.PrimitiveComponent))
  (Variables|Default|SetGhostMat_Inst _returnvalue)
  (bind _returnvalue_2 (Rendering|Material|CreateDynamicMaterialInstance (Variables|Default|GetOccluder) 0 "/Game/Assets/Materials/DepthMask.DepthMask" :!class /Script/Engine.PrimitiveComponent))
  (Variables|Default|SetOcclusionMat_Inst _returnvalue_2))