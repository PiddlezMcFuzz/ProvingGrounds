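; CaveGrid is a modular cave tile actor that builds its own walls in the construction script, leaving sides open toward neighbouring tiles.
; For each wall slot, DirectionCheck box-overlaps around the floor's center socket for other CaveGrid actors and compares their look-at yaw to the flipped wall yaw, within a tolerance.
; A match clears that wall's mesh; otherwise it gets a random mesh from StaticMeshArray.
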(event EventBeginPlay)

(event Collision|EventActorBeginOverlap
  (params (OtherActor :type Actor%20Object%20Reference)))

(event EventTick
  (params (DeltaSeconds :type Float%20%28single-precision%29)))

(fn ConstructionScript
  (bind _y_ (Variables|Default|GetY-))
  (bind _x_ (Variables|Default|GetX+))
  (bind _y__2 (Variables|Default|GetY+))
  (bind _x__2 (Variables|Default|GetX-))
  (bind _output_get (Variables|Default|SetWallMeshIndex (Utilities|Array|MakeArray _x__2 _y_ _x_ _y__2)))
  (Variables|Default|SetWallRot (Utilities|Array|MakeArray (Variables|/Script/Engine.SceneComponent|GetRelativeRotation _x__2) (Variables|/Script/Engine.SceneComponent|GetRelativeRotation _y_) (Variables|/Script/Engine.SceneComponent|GetRelativeRotation _x_) (Variables|/Script/Engine.SceneComponent|GetRelativeRotation _y__2)))
  (for (_array_element _array_index) _output_get
    (bind _collide (CallFunction|DirectionCheck (Variables|Default|GetFloor) _array_index))
    (if _collide
      (Components|StaticMesh|SetStaticMesh _array_element 0)
      (else
        (Components|StaticMesh|SetStaticMesh _array_element (Utilities|Array|Get(acopy) (Variables|Default|GetStaticMeshArray) (Math|Random|RandomInteger 3)))))))

(fn DirectionCheck
  (params (Floor :type Static%20Mesh%20Component%20Object%20Reference) (WallIndex :type Integer))
  (bind _returnvalue (Transformation|GetSocketLocation Floor "center"))
  (LocalVariables|SetWillCollide false)
  (bind _outactors (Collision|BoxOverlapActors _returnvalue "100.000000,100.000000,0.000000" (Utilities|Array|MakeArray "ObjectTypeQuery1" "ObjectTypeQuery2" "ObjectTypeQuery3" "ObjectTypeQuery4") "CaveGrid_C" (Utilities|Array|MakeArray self) :!class /Script/Engine.KismetSystemLibrary))
  (bind _array_element (Utilities|Array|ForEachLoopwithBreak _outactors :!label _label)
    (:LoopBody
      (bind _ascave_grid (Utilities|Casting|CastToCaveGrid _array_element))
      (if (Math|Float|NearlyEqual(Float) (Class|KismetMathLibrary|ClampAxis (.yaw (Math|Rotator|FindLookatRotation _returnvalue (Transformation|GetSocketLocation (Variables|CaveGrid_C|GetFloor _ascave_grid) "center")))) (Class|KismetMathLibrary|ClampAxis (+ (.yaw (Utilities|Array|Get(acopy) (Variables|Default|GetWallRot) WallIndex)) 1.8e+02)) 5.0)
        (bind _output_get (LocalVariables|SetWillCollide true))
        (goto _label Break)))
    (:Completed
      (Development|PrintString (Class|KismetStringLibrary|BuildStringBool (Utilities|String|BuildString(Object) (Utilities|String|BuildString(Object) "" " " self " ") " " (Utilities|Array|Get(acopy) (Variables|Default|GetWallMeshIndex) WallIndex) " collide is ") "" _output_get) false true "(R=0.000000,G=0.660000,B=1.000000,A=1.000000)" 3e+01)
      (return _output_get))))