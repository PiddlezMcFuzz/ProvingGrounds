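; Buoyancy component that floats its owner on the waves of an OceanManager, found automatically at BeginPlay if unset.
; Each tick, a physics-simulating first primitive gets vertical impulses at test points, derived from wave height, buoyancy and cubed depth falloff.
; Gravity switches off while any point is submerged, and damping is raised by total test point count.
; Without physics, the actor snaps to the wave surface around its start location.
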(event EventTick
  (params (DeltaSeconds :type Float%20%28single-precision%29))
  (CallFunction|SimulateBuoyancy (Utilities|Array|Get(acopy) (Actor|GetComponentsByClass (Components|GetOwner) "/Script/Engine.PrimitiveComponent"))))

(event EventBeginPlay
  (Utilities|FlowControl|Sequence
    (:then_0
      ;[1 1 1] Automatically get OceanManager if none specified
      (Utilities|IsValid (Variables|Ocean|GetOceanManager)
        (:Is%20Not%20Valid
          (bind _outactors (Actor|GetAllActorsOfClass "/Game/Salvo/Blueprint/environment/OceanManager.OceanManager_C"))
          (Utilities|IsValid (Utilities|Array|Get(acopy) _outactors)
            (:Is%20Valid
              (Variables|Ocean|SetOceanManager (Utilities|Array|Get(acopy) _outactors)))))))
    (:then_1
      ;[1 1 1] Set Anchor Location
      (Variables|Misc|SetAnchorLocation (Transformation|GetActorLocation (Components|GetOwner))))))

(fn SimulateBuoyancy
  (params (PrimitiveComponent :type Primitive%20Component%20Object%20Reference))
  (bind _returnvalue (Components|GetOwner))
  (bind _gravity (Variables|Misc|GetGravity))
  (bind _testpoints (Variables|Buoyancy|GetTestPoints))
  (bind _returnvalue_2 (Utilities|Array|Length _testpoints))
  (Utilities|IsValid PrimitiveComponent
    (:Is%20Valid
      (if (Physics|IsSimulatingPhysics PrimitiveComponent "None")
        ;[1 1 1] Setup
        (LocalVariables|SetComponent PrimitiveComponent)
        (LocalVariables|SetWorldTransform (Transformation|GetWorldTransform PrimitiveComponent))
        (LocalVariables|SetTestPointCount _returnvalue_2)
        (Utilities|Array|Resize (Variables|Buoyancy|GetTestpoint%20Strengths) _returnvalue_2)
        (LocalVariables|SetHasPointsUnderWater false)
        (Variables|Default|SetTestPoints_Underwater 0)
        (for (_array_element _array_index) (Variables|Buoyancy|GetTestPoints)
          (LocalVariables|Settestpoint%20index _array_index)
          ;[1 1 1] Test point to water surface
          (LocalVariables|SetTestPointWorldSpace (Math|Transform|TransformLocation (LocalVariables|GetWorldTransform) _array_element))
          (bind _delta (Default|GetWaveHeight (Variables|Ocean|GetOceanManager) (Math|Transform|TransformLocation (LocalVariables|GetWorldTransform) _array_element) (Utilities|Time|GetGameTimeinSeconds)))
          (LocalVariables|SetDelta (Math|Float|Clamp(Float) (Math|Float|Absolute(Float) (/ (- (.Z (Math|Vector|BreakVector _delta)) (.Z (Math|Vector|BreakVector (Math|Transform|TransformLocation (LocalVariables|GetWorldTransform) _array_element)))) (Variables|Buoyancy|GetTestPointRadius)))))
          (if (< (- (.Z (Math|Vector|BreakVector _delta)) (.Z (Math|Vector|BreakVector (Math|Transform|TransformLocation (LocalVariables|GetWorldTransform) _array_element)))) 0.0)
            ;[1 1 1] Over Water
            (LocalVariables|SetForce _gravity)
            (else
              ;[1 1 1] Under Water
              (LocalVariables|SetForce (* _gravity (Math|Float|Absolute(Float) (- (Math|Float|Clamp(Float) (+ (Variables|Buoyancy|GetBuoyancy) 1.0) 0.0 2.0) (Utilities|Array|Get(acopy) (Variables|Buoyancy|GetLocalBuoyancies) (LocalVariables|Gettestpoint%20index)))) (* (/ (- (Math|Float|Clamp(Float) (+ (Variables|Buoyancy|GetBuoyancy) 1.0) 0.0 2.0) (Utilities|Array|Get(acopy) (Variables|Buoyancy|GetLocalBuoyancies) (LocalVariables|Gettestpoint%20index))) (Math|Float|Absolute(Float) (- (Math|Float|Clamp(Float) (+ (Variables|Buoyancy|GetBuoyancy) 1.0) 0.0 2.0) (Utilities|Array|Get(acopy) (Variables|Buoyancy|GetLocalBuoyancies) (LocalVariables|Gettestpoint%20index))))) -1.0)))
              (LocalVariables|SetHasPointsUnderWater true)
              (Variables|Default|SetTestPoints_Underwater (+ (Variables|Default|GetTestPoints_Underwater) 1))))
          (Utilities|Array|SetArrayElem (Variables|Buoyancy|GetTestpoint%20Strengths) (LocalVariables|Gettestpoint%20index) (* (Math|Float|Absolute(Float) (- (Math|Float|Clamp(Float) (+ (Variables|Buoyancy|GetBuoyancy) 1.0) 0.0 2.0) (Utilities|Array|Get(acopy) (Variables|Buoyancy|GetLocalBuoyancies) (LocalVariables|Gettestpoint%20index)))) (* (/ (- (Math|Float|Clamp(Float) (+ (Variables|Buoyancy|GetBuoyancy) 1.0) 0.0 2.0) (Utilities|Array|Get(acopy) (Variables|Buoyancy|GetLocalBuoyancies) (LocalVariables|Gettestpoint%20index))) (Math|Float|Absolute(Float) (- (Math|Float|Clamp(Float) (+ (Variables|Buoyancy|GetBuoyancy) 1.0) 0.0 2.0) (Utilities|Array|Get(acopy) (Variables|Buoyancy|GetLocalBuoyancies) (LocalVariables|Gettestpoint%20index))))) -1.0)))
          (if (>= (LocalVariables|GetDelta) 1.0)
            ;[1 1 1] Apply Full or Partial Force
            (LocalVariables|SetForce (/ (LocalVariables|GetForce) (Math|Conversions|ToFloat(Integer) (LocalVariables|GetTestPointCount))))
            (else
              (LocalVariables|SetForce (/ (* (LocalVariables|GetForce) (LocalVariables|GetDelta) (LocalVariables|GetDelta) (LocalVariables|GetDelta)) (Math|Conversions|ToFloat(Integer) (LocalVariables|GetTestPointCount))))))
          ;[1 1 1] Add Impulse
          (Physics|AddImpulseatLocation (LocalVariables|GetComponent) (Math|Vector|MakeVector 0.0 0.0 (LocalVariables|GetForce)) (LocalVariables|GetTestPointWorldSpace) "None"))
        (Physics|SetEnableGravity (LocalVariables|GetComponent) (not (LocalVariables|GetHasPointsUnderWater)))
        ;[1 1 1] Save original Damping Values
        (if (Variables|Misc|GetBaseDampingSet)
          _
          (else
            (Variables|Misc|SetBaseAngularDamping (Class|PrimitiveComponent|GetAngularDamping (LocalVariables|GetComponent)))
            (Variables|Misc|SetBaseLinearDamping (Class|PrimitiveComponent|GetLinearDamping (LocalVariables|GetComponent)))))
        ;[1 1 1] Vary Damping based on number of points underwater
        (Class|PrimitiveComponent|SetLinearDamping (LocalVariables|GetComponent) (+ (* (LocalVariables|GetTestPointCount) 0.1) (Variables|Misc|GetBaseLinearDamping)))
        (Class|PrimitiveComponent|SetAngularDamping (LocalVariables|GetComponent) (+ (* (LocalVariables|GetTestPointCount) 0.25) (Variables|Misc|GetBaseAngularDamping)))
        (else
          ;[1 1 1] No physics snap to water surface
          (bind _delta_2 (Default|GetWaveHeight (Variables|Ocean|GetOceanManager) (Transformation|GetActorLocation _returnvalue) (Utilities|Time|GetGameTimeinSeconds) :!label _label))
          (Transformation|SetActorLocation _returnvalue (Math|Vector|MakeVector (.X (Math|Vector|BreakVector (+ (Variables|Misc|GetAnchorLocation) _delta_2))) (.Y (Math|Vector|BreakVector (+ (Variables|Misc|GetAnchorLocation) _delta_2))) (.Z (Math|Vector|BreakVector _delta_2))) false false))))
    (:Is%20Not%20Valid
      (goto _label))))