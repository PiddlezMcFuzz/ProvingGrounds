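; Debug actor that visualizes OceanManager wave heights as red spheres, for checking alignment with the ocean.
; The construction script finds an OceanManager if none is set and builds a centered grid of local test points from GridCount and Size.
; Tick, throttled by a short Delay, transforms the points with the actor's Z location zeroed, samples GetWaveHeight at game time and draws brief debug spheres at the resulting heights.
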(event EventTick
  (params (DeltaSeconds :type Float%20%28single-precision%29))
  (bind _returnvalue (Transformation|GetActorTransform))
  (Utilities|FlowControl|Delay 0.05)
  (for _array_element (Variables|Default|GetTestPoints)
    (bind _delta (Default|GetWaveHeight (Variables|GridSize|GetOceanManager) (Math|Transform|TransformLocation (Math|Transform|MakeTransform (* (.location _returnvalue) "1.000000,1.000000, 0") (.rotation _returnvalue) (.scale _returnvalue)) _array_element) (Utilities|Time|GetGameTimeinSeconds)))
    (Rendering|Debug|DrawDebugSphere (Math|Vector|MakeVector (.X (Math|Vector|BreakVector (Math|Transform|TransformLocation (Math|Transform|MakeTransform (* (.location _returnvalue) "1.000000,1.000000, 0") (.rotation _returnvalue) (.scale _returnvalue)) _array_element))) (.Y (Math|Vector|BreakVector (Math|Transform|TransformLocation (Math|Transform|MakeTransform (* (.location _returnvalue) "1.000000,1.000000, 0") (.rotation _returnvalue) (.scale _returnvalue)) _array_element))) (- (.Z (Math|Vector|BreakVector _delta)) (.Z (Math|Vector|BreakVector (Math|Transform|TransformLocation (Math|Transform|MakeTransform (* (.location _returnvalue) "1.000000,1.000000, 0") (.rotation _returnvalue) (.scale _returnvalue)) _array_element))))) 5e+01 5 "(R=1.000000,G=0.000000,B=0.000000,A=1.000000)" 0.06)))

(fn ConstructionScript
  (bind _size (Variables|GridSize|GetSize))
  (bind _grid_count (Variables|GridSize|GetGrid%20Count))
  (bind _returnvalue (/ _grid_count 2))
  (bind _returnvalue_2 (- 0 _returnvalue))
  (Utilities|FlowControl|Sequence
    (:then_0
      (Utilities|IsValid (Variables|GridSize|GetOceanManager)
        (:Is%20Not%20Valid
          (bind _outactors (Actor|GetAllActorsOfClass "/Game/Salvo/Blueprint/environment/OceanManager.OceanManager_C"))
          (Utilities|IsValid (Utilities|Array|Get(acopy) _outactors)
            (:Is%20Valid
              (Variables|GridSize|SetOceanManager (Utilities|Array|Get(acopy) _outactors)))))))
    (:then_1
      (for _index (range _returnvalue_2 _returnvalue)
        (for _index_2 (range _returnvalue_2 _returnvalue)
          (Utilities|Array|Add (Variables|Default|GetTestPoints) (Math|Vector|MakeVector (* _index _size) (* _index_2 _size) 0.0)))))))